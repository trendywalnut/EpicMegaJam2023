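; Merchant logic Blueprint that generates customer dice rolls, scaled by a rising difficulty modifier.
; On BeginPlay it picks a d4 to d10 through cascaded weighted branches, rolls it, and adds an occasional positive or negative mood bonus.
; It multiplies and rounds the total, prints it, then re-enters selection after a short delay, looping endlessly.
; A separate event raises the difficulty modifier, but nothing here calls it.
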(event `Key|One`
  (params (Key :type "Key Structure")))

(event `Key|Two`
  (params (Key :type "Key Structure")))

(event `Key|Three`
  (params (Key :type "Key Structure")))

(event `Increase Difficulty Mod`
  ;[1 1 1] Up the Difficulty Mod for variety
  (set `self.DifficultyMod` (+ (`self.DifficultyMod`) 0.3)))

(event `self.ReceiveBeginPlay`
  (`/Engine/EditorBlueprintResources/StandardMacros.DoOnce` false
    (:`Completed`
      (set `self.DifficultyMod` 1.0)
      ;[0.3105 1 0.2592] Customer Die Selected
      (if (`KismetMathLibrary.RandomBoolWithWeight` 0.16) :!label _label
        (bind _output_get (set `self.CustomerDie` 10))
        (`self.Customer Dice Roll` _output_get)
        (elif (`KismetMathLibrary.RandomBoolWithWeight` 0.33)
          (bind _output_get_2 (set `self.CustomerDie` 8))
          (`self.Customer Dice Roll` _output_get_2)
          (elif (`KismetMathLibrary.RandomBoolWithWeight` 0.5)
            (bind _output_get_3 (set `self.CustomerDie` 6)) ; customer die is 1d6
            (`self.Customer Dice Roll` _output_get_3)
            (else
              (bind _output_get_4 (set `self.CustomerDie` 4)) ; customer die is 1d4
              (`self.Customer Dice Roll` _output_get_4)))))
      (if true
        ;[0.333 1 0.9801] Customer Random Status
        (if (`KismetMathLibrary.RandomBoolWithWeight` 0.33)
          (if (`KismetMathLibrary.RandomBoolWithWeight` 0.66)
            (bind _returnvalue (`self.Random Bonus Generation`)) ; positive bonus
            (set `self.CustomerMoodBonus` _returnvalue)
            (else
              (bind _returnvalue_2 (`self.Random Bonus Generation`)) ; negative bonus
              (set `self.CustomerMoodBonus` (* _returnvalue_2 -1))))
          (else
            (set `self.CustomerMoodBonus` 0) ; Customer has no bonus
          ))
        (bind _output_get_5 (set `self.CustomerDieRoll` (`KismetMathLibrary.Round` (* (+ (`self.CustomerMoodBonus`) (`self.CustomerDieRoll`)) (`self.DifficultyMod`))))) ; final customer roll result
        (`KismetSystemLibrary.PrintString` (`KismetStringLibrary.Conv_IntToString` _output_get_5))
        (`KismetSystemLibrary.Delay` 0.5)
        (`self.Customer Dice Selection`)))))

(event `Customer Dice Selection`
  ;[0.3105 1 0.2592] Customer Die Selected
  (goto _label))

(event `Customer Dice Roll`
  (params (DiceMax :type Integer))
  ;[0.6927 0.3854 1] Customer Dice Roll Function
  (set `self.CustomerDieRoll` (`KismetMathLibrary.RandomIntegerInRange` 1 DiceMax)))

(fn `NewFunction`)

(fn `Random Bonus Generation`
  (returns (ReturnValue :type Integer))
  (return (`KismetMathLibrary.SelectInt` 1 (`KismetMathLibrary.SelectInt` 3 2 (`KismetMathLibrary.RandomBoolWithWeight` 0.33)) (`KismetMathLibrary.RandomBoolWithWeight` 0.5))))